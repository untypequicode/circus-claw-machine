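; BP_Balles moves its Scene component on three input axes, apparently as the claw of a claw machine.
; While NewVar0 is true, each axis input offsets the relative location, with SelectFloat keeping the old value whenever the new one leaves fixed bounds.
; The forward and vertical checks also block a low region at the front of the range.
; The right/left event still prints a debug "Hello".
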(event EventBeginPlay)

(event Collision|EventActorBeginOverlap
  (params (OtherActor :type Actor%20Object%20Reference)))

(event EventTick
  (params (DeltaSeconds :type Float%20%28single-precision%29)))

(event Input|AxisEvents|InputAxisMoveForward/Backward
  (params (AxisValue :type Float%20%28single-precision%29))
  (bind _returnvalue (* AxisValue 1.0))
  (bind _scene (Variables|Default|GetScene))
  (bind _relativelocation (Variables|/Script/Engine.SceneComponent|GetRelativeLocation _scene))
  (bind _returnvalue_2 (+ _returnvalue (.x _relativelocation)))
  ;[1 1 1] Move Forward / Backward
  (if (Variables|Default|GetNewVar_0)
    (Transformation|SetRelativeLocation _scene (Math|Vector|MakeVector (Math|Float|SelectFloat _returnvalue_2 (.x _relativelocation) (Math|Boolean|ANDBoolean (<= _returnvalue_2 34.0) (>= _returnvalue_2 -34.0) (not (and (<= (.z _relativelocation) 98.0) (>= _returnvalue_2 2e+01))))) (.y _relativelocation) (.z _relativelocation)) false false)))

(event Input|AxisEvents|InputAxisClawAxeZ
  (params (AxisValue :type Float%20%28single-precision%29))
  (bind _scene (Variables|Default|GetScene))
  (bind _relativelocation (Variables|/Script/Engine.SceneComponent|GetRelativeLocation _scene))
  (bind _returnvalue (+ (.z _relativelocation) AxisValue))
  ;[1 1 1] Move Axe Z
  (if (Variables|Default|GetNewVar_0)
    (Transformation|SetRelativeLocation _scene (Math|Vector|MakeVector (.x _relativelocation) (.y _relativelocation) (Math|Float|SelectFloat _returnvalue (.z _relativelocation) (Math|Boolean|ANDBoolean (<= _returnvalue 105.0) (>= _returnvalue 38.0) (not (and (<= _returnvalue 98.0) (>= (.x _relativelocation) 2e+01)))))) false false)))

(event Input|AxisEvents|InputAxisMoveRight/Left
  (params (AxisValue :type Float%20%28single-precision%29))
  (bind _returnvalue (* AxisValue -1.0))
  (bind _scene (Variables|Default|GetScene))
  (bind _relativelocation (Variables|/Script/Engine.SceneComponent|GetRelativeLocation _scene))
  (bind _returnvalue_2 (+ _returnvalue (.y _relativelocation)))
  ;[1 1 1] Move Right / Left
  (Development|PrintString "Hello")
  (if (Variables|Default|GetNewVar_0)
    (Transformation|SetRelativeLocation _scene (Math|Vector|MakeVector (.x _relativelocation) (Math|Float|SelectFloat _returnvalue_2 (.y _relativelocation) (and (<= _returnvalue_2 34.0) (>= _returnvalue_2 -34.0))) (.z _relativelocation)) false false)))

(fn ConstructionScript)