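; BP_Box is a sliding target that turns BP_Balles overlaps into saved choices or menu actions, stopping after three balls.
; Each overlap creates a fresh BP_transition save and switches on ball type: mechanic types overwrite slot "partie", while Random picks one without saving.
; A third mechanic ball, or any Play ball, opens Level0 after a delay; Quitter exits.
; Tick bounces the Scene component along Y.
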(event OnComponentBeginOverlap(Box)
  (params (OverlappedComponent :type Primitive%20Component%20Object%20Reference) (OtherActor :type Actor%20Object%20Reference) (OtherComp :type Primitive%20Component%20Object%20Reference) (OtherBodyIndex :type Integer) (bFromSweep :type Boolean) (SweepResult :type Hit%20Result%20Structure%20%28by%20ref%29))
  (Utilities|Casting|CastToBP_Balles OtherActor)
  (Development|PrintString "Hello"))

(event EventBeginPlay)

(event Collision|EventActorBeginOverlap
  (params (OtherActor :type Actor%20Object%20Reference))
  (bind _asbp_balles (Utilities|Casting|CastToBP_Balles OtherActor))
  (bind _output_get (Variables|Default|Setcombien (+ (Variables|Default|Getcombien) 1)))
  (bind _returnvalue (SaveGame|CreateSaveGameObject "/Game/Blueprint/BP_transition.BP_transition_C"))
  (switch Utilities|FlowControl|Switch|SwitchonEnum_billes (Variables|/Game/Blueprint/BP_Balles.BP_Balles_C|Getenum_bille _asbp_balles)
    (:NewEnumerator0
      (Utilities|Array|Add (Variables|/Game/Blueprint/BP_transition.BP_transition_C|Getnomvariable _returnvalue) (Variables|/Game/Blueprint/BP_Balles.BP_Balles_C|Getenum_bille _asbp_balles) :!label _label)
      (SaveGame|SaveGametoSlot _returnvalue "partie")
      (Development|PrintString (Utilities|String|EnumtoString (Variables|/Game/Blueprint/BP_Balles.BP_Balles_C|Getenum_bille _asbp_balles)))
      (if (>= _output_get 3)
        (Development|PrintString "The game will start" :!label _label_2)
        (Utilities|FlowControl|Delay 5.0)
        (Game|OpenLevel(byName) "Level0")))
    (:NewEnumerator1
      (goto _label))
    (:NewEnumerator2
      (goto _label))
    (:NewEnumerator3
      (goto _label))
    (:NewEnumerator4
      (goto _label))
    (:NewEnumerator5
      (switch Utilities|FlowControl|Switch|SwitchonEnum_Balle (.OutItem (Utilities|Array|Random (Variables|Default|Getrandom)))
        (:NewEnumerator0
          (Utilities|Array|Add (Variables|/Game/Blueprint/BP_transition.BP_transition_C|Getnomvariable _returnvalue) "NewEnumerator0")
          (Development|PrintString "SwitchBasic"))
        (:NewEnumerator1
          (Utilities|Array|Add (Variables|/Game/Blueprint/BP_transition.BP_transition_C|Getnomvariable _returnvalue) "NewEnumerator1")
          (Development|PrintString "SwitchAlt"))
        (:NewEnumerator2
          (Utilities|Array|Add (Variables|/Game/Blueprint/BP_transition.BP_transition_C|Getnomvariable _returnvalue) "NewEnumerator2")
          (Development|PrintString "Gravity"))
        (:NewEnumerator3
          (Utilities|Array|Add (Variables|/Game/Blueprint/BP_transition.BP_transition_C|Getnomvariable _returnvalue) "NewEnumerator3")
          (Development|PrintString "Rotate"))
        (:NewEnumerator4
          (Utilities|Array|Add (Variables|/Game/Blueprint/BP_transition.BP_transition_C|Getnomvariable _returnvalue) "NewEnumerator4")
          (Development|PrintString "Missclick"))))
    (:NewEnumerator6
      (Utilities|FlowControl|Delay 5.0)
      (Game|QuitGame 0 "Quit" false))
    (:NewEnumerator7
      (goto _label_2))))

(event EventTick
  (params (DeltaSeconds :type Float%20%28single-precision%29))
  (bind _scene (Variables|Default|GetScene))
  (bind _relativelocation (Variables|/Script/Engine.SceneComponent|GetRelativeLocation _scene))
  (if (< (Variables|Default|Getcombien) 3)
    (Transformation|SetRelativeLocation _scene (Math|Vector|MakeVector 0.0 (+ (* 1e+01 DeltaSeconds (Math|Float|SelectFloat 1.0 -1.0 (Variables|Default|Getplus_location))) (.y _relativelocation)) 0.0) false false)
    (if (or (>= (.y _relativelocation) 35.0) (<= (.y _relativelocation) -35.0))
      (Variables|Default|Setplus_location (not (Variables|Default|Getplus_location))))))

(fn ConstructionScript)