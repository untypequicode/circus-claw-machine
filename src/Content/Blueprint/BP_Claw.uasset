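; BP_Claw is a player-controlled claw that moves within a bounded box, driven by input axes.
; Forward/back, right/left and claw_down axes each offset the Scene component's relative location on X, Y or Z, using SelectFloat to reject out-of-range steps.
; Extra checks on X and Z keep the lowered claw out of the forward end of the box.
; The Sphere overlap event is an empty stub.
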(event OnComponentBeginOverlap(Sphere)
  (params (OverlappedComponent :type Primitive%20Component%20Object%20Reference) (OtherActor :type Actor%20Object%20Reference) (OtherComp :type Primitive%20Component%20Object%20Reference) (OtherBodyIndex :type Integer) (bFromSweep :type Boolean) (SweepResult :type Hit%20Result%20Structure%20%28by%20ref%29)))

(event EventBeginPlay
  (Transformation|SetRelativeLocation (Variables|Default|GetScene) (Math|Vector|MakeVector 0.0 0.0 0.0) false false))

(event Collision|EventActorBeginOverlap
  (params (OtherActor :type Actor%20Object%20Reference)))

(event EventTick
  (params (DeltaSeconds :type Float%20%28single-precision%29)))

(event Input|AxisEvents|InputAxisMoveForward/Backward
  (params (AxisValue :type Float%20%28single-precision%29))
  (bind _returnvalue (* AxisValue 2.0))
  (bind _scene (Variables|Default|GetScene))
  (bind _relativelocation (Variables|/Script/Engine.SceneComponent|GetRelativeLocation _scene))
  (bind _returnvalue_2 (+ _returnvalue (.x _relativelocation)))
  (Transformation|SetRelativeLocation _scene (Math|Vector|MakeVector (Math|Float|SelectFloat _returnvalue_2 (.x _relativelocation) (Math|Boolean|ANDBoolean (<= _returnvalue_2 34.0) (>= _returnvalue_2 -34.0) (not (and (<= (.z _relativelocation) -2.0) (>= _returnvalue_2 2e+01))))) (.y _relativelocation) (.z _relativelocation)) false false))

(event Input|AxisEvents|InputAxisMoveRight/Left
  (params (AxisValue :type Float%20%28single-precision%29))
  (bind _returnvalue (* AxisValue -2.0))
  (bind _scene (Variables|Default|GetScene))
  (bind _relativelocation (Variables|/Script/Engine.SceneComponent|GetRelativeLocation _scene))
  (bind _returnvalue_2 (+ _returnvalue (.y _relativelocation)))
  (Transformation|SetRelativeLocation _scene (Math|Vector|MakeVector (.x _relativelocation) (Math|Float|SelectFloat _returnvalue_2 (.y _relativelocation) (and (<= _returnvalue_2 34.0) (>= _returnvalue_2 -34.0))) (.z _relativelocation)) false false))

(event Input|AxisEvents|InputAxisclaw_down
  (params (AxisValue :type Float%20%28single-precision%29))
  (bind _scene (Variables|Default|GetScene))
  (bind _relativelocation (Variables|/Script/Engine.SceneComponent|GetRelativeLocation _scene))
  (bind _returnvalue (+ (.z _relativelocation) AxisValue))
  (Transformation|SetRelativeLocation _scene (Math|Vector|MakeVector (.x _relativelocation) (.y _relativelocation) (Math|Float|SelectFloat _returnvalue (.z _relativelocation) (Math|Boolean|ANDBoolean (<= _returnvalue 5.0) (>= _returnvalue -57.0) (not (and (<= _returnvalue -2.0) (>= (.x _relativelocation) 2e+01)))))) false false))

(fn ConstructionScript)