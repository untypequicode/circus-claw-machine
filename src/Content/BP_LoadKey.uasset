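; Actor that remaps movement, jump and claw-axis keys at BeginPlay according to the keyboard layout (QWERTY or AZERTY) stored in the "config" save.
; If that save exists, the saved layout selects which W/Z and Q/A keys to swap.
; SwapAction and SwapAxis remove and re-add mappings in the global Input Settings, then update a key collection on Keyboard.
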(event EventBeginPlay
  (bind _returnvalue (SaveGame|DoesSaveGameExist "config"))
  (if _returnvalue
    (bind _returnvalue_2 (SaveGame|LoadGamefromSlot "config"))
    (bind _asbp_save_config (Utilities|Casting|CastToBP_SaveConfig _returnvalue_2))
    (CallFunction|SwapAction (Utilities|Struct|MakeInputActionKeyMapping "Jump" false false false false (Utilities|Select :Index (Variables|/Game/Blueprint/BP_SaveConfig.BP_SaveConfig_C|GetKeyboard _asbp_save_config) :NewEnumerator0 "W" :NewEnumerator1 "Z")) (Utilities|Select :Index (Variables|/Game/Blueprint/BP_SaveConfig.BP_SaveConfig_C|GetKeyboard _asbp_save_config) :NewEnumerator0 "Z" :NewEnumerator1 "W"))
    (CallFunction|SwapAxis (Utilities|Struct|MakeInputAxisKeyMapping "Move Forward / Backward" 1.0 (Utilities|Select :Index (Variables|/Game/Blueprint/BP_SaveConfig.BP_SaveConfig_C|GetKeyboard _asbp_save_config) :NewEnumerator0 "W" :NewEnumerator1 "Z")) (Utilities|Select :Index (Variables|/Game/Blueprint/BP_SaveConfig.BP_SaveConfig_C|GetKeyboard _asbp_save_config) :NewEnumerator0 "Z" :NewEnumerator1 "W"))
    (CallFunction|SwapAxis (Utilities|Struct|MakeInputAxisKeyMapping "Move Right / Left" 1.0 (Utilities|Select :Index (Variables|/Game/Blueprint/BP_SaveConfig.BP_SaveConfig_C|GetKeyboard _asbp_save_config) :NewEnumerator0 "Q" :NewEnumerator1 "A")) (Utilities|Select :Index (Variables|/Game/Blueprint/BP_SaveConfig.BP_SaveConfig_C|GetKeyboard _asbp_save_config) :NewEnumerator0 "A" :NewEnumerator1 "Q"))
    (CallFunction|SwapAxis (Utilities|Struct|MakeInputAxisKeyMapping "Claw Axe Z" 1.0 (Utilities|Select :Index (Variables|/Game/Blueprint/BP_SaveConfig.BP_SaveConfig_C|GetKeyboard _asbp_save_config) :NewEnumerator0 "Q" :NewEnumerator1 "A")) (Utilities|Select :Index (Variables|/Game/Blueprint/BP_SaveConfig.BP_SaveConfig_C|GetKeyboard _asbp_save_config) :NewEnumerator0 "A" :NewEnumerator1 "Q"))))

(event Collision|EventActorBeginOverlap
  (params (OtherActor :type Actor%20Object%20Reference)))

(event EventTick
  (params (DeltaSeconds :type Float%20%28single-precision%29)))

(fn ConstructionScript)

(fn SwapAction
  (params (Action :type Input%20Action%20Key%20Mapping%20Structure) (Key :type Key%20Structure :default "None"))
  (bind (_actionname _bshift _bctrl _balt _bcmd _key) (Utilities|Struct|BreakInputActionKeyMapping Action))
  (bind _returnvalue (Class|InputSettings|GetInputSettings))
  (bind _keyboard (LocalVariables|GetKeyboard))
  (bind _membervar_0 (Utilities|Struct|BreakStruct_keyboard _keyboard))
  (Class|InputSettings|RemoveActionMapping _returnvalue Action true)
  (Class|InputSettings|AddActionMapping _returnvalue (Utilities|Struct|MakeInputActionKeyMapping _actionname _bshift _bctrl _balt _bcmd Key) true)
  (Utilities|Array|RemoveItem _membervar_0 _key)
  (Utilities|Array|Add _membervar_0 Key))

(fn SwapAxis
  (params (Axis :type Input%20Axis%20Key%20Mapping%20Structure) (Key :type Key%20Structure :default "None"))
  (bind (_axisname _scale _key) (Utilities|Struct|BreakInputAxisKeyMapping Axis))
  (bind _returnvalue (Class|InputSettings|GetInputSettings))
  (bind _keyboard (LocalVariables|GetKeyboard))
  (bind _membervar_0 (Utilities|Struct|BreakStruct_keyboard _keyboard))
  (Class|InputSettings|RemoveAxisMapping _returnvalue Axis true)
  (Class|InputSettings|AddAxisMapping _returnvalue (Utilities|Struct|MakeInputAxisKeyMapping _axisname _scale Key) true)
  (Utilities|Array|RemoveItem _membervar_0 _key)
  (Utilities|Array|Add _membervar_0 Key))